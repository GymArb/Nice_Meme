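; BP_6DOF_Pawn is a player-controlled pawn that flies with six-degree-of-freedom style controls.
; Forward and right axes set BodyMesh's physics linear velocity along the actor's own vectors, with no separate vertical axis.
; Each movement write replaces the current velocity, so the two axes overwrite each other instead of combining.
; LookUp, Turn and Rotate apply unscaled local pitch, yaw and roll to the actor.
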(event Input|AxisEvents|InputAxisMoveRight
  (params (AxisValue :type Float%20%28single-precision%29))
  (Physics|SetPhysicsLinearVelocity (Variables|Default|GetBodyMesh) (* (Math|Vector|GetRightVector (Transformation|GetActorRotation)) (* AxisValue 1e+02)) false "None"))

(event Input|AxisEvents|InputAxisRotate
  (params (AxisValue :type Float%20%28single-precision%29))
  (Transformation|AddActorLocalRotation (Math|Rotator|MakeRotator AxisValue 0.0 0.0) false false))

(event Input|AxisEvents|InputAxisLookUp
  (params (AxisValue :type Float%20%28single-precision%29))
  (Transformation|AddActorLocalRotation (Math|Rotator|MakeRotator 0.0 AxisValue 0.0) false false))

(event Input|AxisEvents|InputAxisTurn
  (params (AxisValue :type Float%20%28single-precision%29))
  (Transformation|AddActorLocalRotation (Math|Rotator|MakeRotator 0.0 0.0 AxisValue) false false))

(event Input|AxisEvents|InputAxisMoveForward
  (params (AxisValue :type Float%20%28single-precision%29))
  (Physics|SetPhysicsLinearVelocity (Variables|Default|GetBodyMesh) (* (Math|Vector|GetForwardVector (Transformation|GetActorRotation)) (* AxisValue 1e+02)) false "None"))

(fn ConstructionScript)